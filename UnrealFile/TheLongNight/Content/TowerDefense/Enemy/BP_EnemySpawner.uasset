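; Tower defense enemy spawner that spawns a wave of enemies at its own transform when SpawnWaves is called.
; SpawnEnemy re-calls itself after a fixed delay until the spawned count reaches one more than the wave number, then resets the counter.
; Each spawn notifies the first player's controller through ChangeEnemiesAliveMessage to update the enemies-alive message.
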(event Custom|Spawn%20Enemy
  (if (== (+ (stale EventSpawnWaves WaveNumber) 1) (Variables|Default|GetEnemiesSpwaned))
    (Variables|Default|SetEnemiesSpwaned 0)
    (else
      (Game|SpawnActorfromClass "/Game/TowerDefense/Enemy/BP_Enemy.BP_Enemy_C" (Transformation|GetActorTransform) "Undefined" "MultiplyWithRoot" 0 0)
      (Variables|Default|SetEnemiesSpwaned (+ (Variables|Default|GetEnemiesSpwaned) 1))
      (Utilities|FlowControl|Sequence
        (:then_0
          (Class|BPIWaves|ChangeEnemiesAlive(Message) (Game|GetPlayerController (Variables|/Script/Engine.Pawn|GetPlayerState (Game|GetPlayerCharacter 0))) true))
        (:then_1
          (Utilities|FlowControl|Delay 3.0)
          (CallFunction|SpawnEnemy))))))

(event EventSpawnWaves
  (params (WaveNumber :type Integer))
  (CallFunction|SpawnEnemy))

(fn ConstructionScript)