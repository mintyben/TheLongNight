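; BP_Enemy is a tower defense enemy that takes damage, shows a floating health bar and dies at zero health.
; Tick updates the health bar widget percentage and rotates the widget component to face the player camera.
; AnyDamage reduces health and calls Death, which tells the player controller to update the enemies-alive message and then destroys the actor.
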(event Custom|Death
  (Class|BPIWaves|ChangeEnemiesAlive(Message) (Game|GetPlayerController (Variables|/Script/Engine.Pawn|GetPlayerState (Game|GetPlayerCharacter 0))) false)
  (Actor|DestroyActor))

(event Game|Damage|EventAnyDamage
  (params (Damage :type Float%20%28single-precision%29) (DamageType :type Damage%20Type%20Object%20Reference) (InstigatedBy :type Controller%20Object%20Reference) (DamageCauser :type Actor%20Object%20Reference))
  (if (> (Variables|Default|GetHealth) 0.0)
    (bind _output_get (Variables|Default|SetHealth (- (Variables|Default|GetHealth) Damage)))
    (if (<= _output_get 0.0)
      (CallFunction|Death))))

(event EventBeginPlay
  (bind _aswb_health_bar (Utilities|Casting|CastToWB_HealthBar (UserInterface|GetUserWidgetObject (Variables|Default|GetEnemyHealthBar))))
  (Variables|Default|SetAs%20WB%20Health%20Bar _aswb_health_bar))

(event EventTick
  (params (DeltaSeconds :type Float%20%28single-precision%29))
  (bind _enemyhealthbar (Variables|Default|GetEnemyHealthBar))
  (Progress|SetPercent (Variables|/Game/TowerDefense/HUD/WB_HealthBar.WB_HealthBar_C|GetHealthBar (Variables|Default|GetAs%20WB%20Health%20Bar)) (/ (Variables|Default|GetHealth) (Variables|Default|GetMax_Health)))
  (Transformation|SetWorldRotation _enemyhealthbar (Math|Rotator|FindLookatRotation (Transformation|GetWorldLocation _enemyhealthbar) (Transformation|GetWorldLocation (Variables|/Script/Engine.PlayerCameraManager|GetTransformComponent (Game|GetPlayerCameraManager 0)))) false false))

(fn ConstructionScript)