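; Catapult tower for a tower defense game that fires projectiles at a target location on a looping timer.
; Clicking it spawns BP_BoomSpot markers at offsets around it, gated against repeat clicks.
; Despawning them reopens the gate, turns the catapult toward CatapultTarget and starts the firing timer.
; It creates an upgrade widget and exposes damage, area and speed upgrades; shot delay is only applied when the timer is set.
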(event Custom|Open%20Gate
  (bind _catapults1 (Variables|Default|GetCatapultS1))
  (bind _catapult_target (Variables|Default|GetCatapult_Target))
  (bind _returnvalue (Transformation|GetWorldLocation _catapults1))
  (bind _returnvalue_2 (Math|Rotator|FindLookatRotation _catapult_target _returnvalue))
  (Utilities|FlowControl|Sequence
    (:then_0
      (Utilities|FlowControl|Gate false) ; enters at Open
    )
    (:then_1
      (Transformation|SetWorldRotation (Variables|Default|GetCatapultS1) (Math|Rotator|MakeRotator (.roll _returnvalue_2) 0.0 (.yaw _returnvalue_2)) false false))
    (:then_2
      (Utilities|Time|SetTimerbyEvent (delegate Custom|Shoot) (Variables|Default|GetShotDelay) true))))

(event Custom|Shoot
  (CallFunction|ShootProjectile (Variables|Default|GetDamage) (Variables|Default|GetArea)))

(event MouseInput|EventActorOnClicked
  (params (ButtonPressed :type Key%20Structure :default "None"))
  (Utilities|FlowControl|Gate false :!label _label
    (:Exit
      (for (_array_element _array_index) (Variables|Default|GetSpawnLocations)
        (CallFunction|SpawnBoomSpots (+ _array_element (Transformation|GetActorLocation)) _array_index))
      (goto _label Close))))

(event EventBeginPlay
  (bind _returnvalue (UserInterface|CreateWidget "/Game/TowerDefense/Towers/CatapultTower/WBP_CatapultUpgrade.WBP_CatapultUpgrade_C" (Game|GetPlayerController 0) self))
  (Variables|Default|SetWBP%20CatapultUpgrade _returnvalue))

(event EventUpgradeArea
  (Variables|Default|SetArea (+ (Variables|Default|GetArea) 5e+02))
  (bind _output_get (Variables|Default|SetUpgradeNum (+ (Variables|Default|GetUpgradeNum) 1)))
  (switch int _output_get))

(event EventUpgradeDamage
  (Variables|Default|SetDamage (+ (Variables|Default|GetDamage) 5.0))
  (bind _output_get (Variables|Default|SetUpgradeNum (+ (Variables|Default|GetUpgradeNum) 1)))
  (switch int _output_get))

(event EventCloseUpgrades
  (Widget|RemovefromParent (Variables|Default|GetWBP%20CatapultUpgrade)))

(event EventUpgradeSpeed
  (Variables|Default|SetShotDelay (- (Variables|Default|GetShotDelay) 0.5))
  (bind _output_get (Variables|Default|SetUpgradeNum (+ (Variables|Default|GetUpgradeNum) 1)))
  (switch int _output_get))

(fn ConstructionScript)

(fn ShootProjectile
  (params (Damage :type Float%20%28double-precision%29) (Area :type Float%20%28double-precision%29))
  (Game|SpawnActorfromClass "/Game/TowerDefense/Towers/CatapultTower/BP_CatapultProjectile.BP_CatapultProjectile_C" (Math|Transform|MakeTransform (Transformation|GetWorldLocation (Variables|Default|Getspawnpoint)) "0, 0, 0" "1.000000,1.000000,1.000000") "Undefined" "MultiplyWithRoot" 0 (Variables|Default|GetCatapult_Target) Damage Area 0))

(fn SpawnBoomSpots
  (params (Boom_Location :type Vector) (Index :type Integer))
  (bind _returnvalue (Game|SpawnActorfromClass "/Game/TowerDefense/Towers/CatapultTower/BP_BoomSpot.BP_BoomSpot_C" (Math|Transform|MakeTransform Boom_Location "0, 0, 0" "1.000000,1.000000,1.000000") "Undefined" "MultiplyWithRoot" 0 self 0))
  (Utilities|Array|SetArrayElem (Variables|Default|GetBoomSpots) Index _returnvalue))

(fn DespawnBoomSpots
  (for _array_element (Variables|Default|GetBoomSpots)
    (Actor|DestroyActor _array_element))
  (CallFunction|OpenGate))