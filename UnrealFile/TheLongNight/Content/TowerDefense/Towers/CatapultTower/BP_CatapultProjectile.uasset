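; Projectile fired by the tower defense catapult tower, lobbed toward a target location to deal area damage.
; On BeginPlay it sets its ProjectileMovement velocity from the direction to TargetLocation, with an upward bias and per-axis scaling to form an arc.
; On overlapping any actor other than BP_Catapult, it applies radial damage at its own location and destroys itself.
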(event EventBeginPlay
  (Variables|/Script/Engine.MovementComponent|SetVelocity (Variables|Default|GetProjectileMovement) (* (+ (Math|Vector|GetUnitDirection(Vector) (Transformation|GetActorLocation) (Variables|Default|GetTarget_Location)) "0.000000,0.000000,2.200000") "400.000000,400.000000,1000.000000")))

(event Collision|EventActorBeginOverlap
  (params (OtherActor :type Actor%20Object%20Reference))
  (if (not (== OtherActor "/Game/TowerDefense/Towers/CatapultTower/BP_Catapult.BP_Catapult"))
    (Game|Damage|ApplyRadialDamage 2e+01 (Transformation|GetActorLocation) 3e+03 0 0 0 0 false "ECC_Visibility")
    (Actor|DestroyActor)))

(fn ConstructionScript)