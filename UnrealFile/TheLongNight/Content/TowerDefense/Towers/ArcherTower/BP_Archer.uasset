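; BP_Archer is a tower defense archer that fires BP_ArcherProjectile when its PawnSensing component sees a BP_Enemy.
; The projectile spawns at the Scene component's transform and targets the first enemy from GetActorOfClass, not necessarily the seen pawn.
; Two chained gates close after each shot: one reopens after a one-second cooldown, the other when ProjectileDestroyed is called, limiting it to one live projectile.
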(event OnSeePawn(PawnSensing)
  (params (Pawn :type Pawn%20Object%20Reference))
  (bind _self self)
  (Utilities|Casting|CastToBP_Enemy Pawn)
  (Utilities|FlowControl|Gate false :!label _label
    (:Exit
      (Utilities|FlowControl|Gate false :!label _label_2
        (:Exit
          (bind _returnvalue (Actor|GetActorOfClass "/Game/TowerDefense/Enemy/BP_Enemy.BP_Enemy_C"))
          (Game|SpawnActorfromClass "/Game/TowerDefense/Towers/ArcherTower/BP_ArcherProjectile.BP_ArcherProjectile_C" (Transformation|GetWorldTransform (Variables|Default|GetScene)) "Undefined" "MultiplyWithRoot" _self _returnvalue _self 0)
          (Utilities|FlowControl|Sequence
            (:then_0
              (goto _label Close))
            (:then_1
              (goto _label_2 Close))
            (:then_2
              (Utilities|FlowControl|Delay 1.0)
              (goto _label Open))))))))

(event EventProjectileDestroyed
  (bind _self self)
  (Utilities|FlowControl|Gate false) ; enters at Open
)

(fn ConstructionScript)