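; Homing projectile for the tower defense Ballista tower that damages the enemy it hits.
; On spawn, if its Target is valid, it sets velocity and rotation toward that target and assigns the target's root as the ProjectileMovement homing component, then self-destructs after a short delay.
; Overlapping any BP_Enemy, not only the target, applies fixed damage and destroys the projectile.
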(event OnComponentBeginOverlap(BallistaProjCollision)
  (params (OverlappedComponent :type Primitive%20Component%20Object%20Reference) (OtherActor :type Actor%20Object%20Reference) (OtherComp :type Primitive%20Component%20Object%20Reference) (OtherBodyIndex :type Integer) (bFromSweep :type Boolean) (SweepResult :type Hit%20Result%20Structure%20%28by%20ref%29))
  (bind _asbp_enemy (Utilities|Casting|CastToBP_Enemy OtherActor))
  (if (== _asbp_enemy OtherActor)
    (Game|Damage|ApplyDamage OtherActor 1e+02 0 0)
    (Actor|DestroyActor)))

(event Custom|Aim%20Projectile
  (bind _output_get (Variables|/Script/Engine.MovementComponent|SetVelocity (Variables|Default|GetProjectileMovement) (Math|Vector|GetUnitDirection(Vector) (Transformation|GetActorLocation) (Transformation|GetActorLocation (Variables|Default|GetTarget)))))
  (Transformation|SetActorRotation (Math|Conversions|RotationFromXVector _output_get))
  (Variables|/Script/Engine.ProjectileMovementComponent|SetHomingTargetComponent (Variables|Default|GetProjectileMovement) (Variables|/Script/Engine.Actor|GetRootComponent (Variables|Default|GetTarget)))
  (Utilities|FlowControl|Delay 3.0)
  (Actor|DestroyActor))

(event EventBeginPlay
  (Variables|Default|GetTarget
    (:then
      (CallFunction|AimProjectile))
    (:else)))

(fn ConstructionScript)